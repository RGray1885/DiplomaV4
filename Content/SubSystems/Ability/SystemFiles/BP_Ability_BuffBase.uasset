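; Base ability actor for buffs, which shows the buff in the player HUD and keeps copies from stacking.
; On BeginPlay it scans the actors attached to its owner, destroying any of its own class and reporting the cleared effect to the player stats subsystem.
; A notification handler leads to CastAbility, which registers the actor with the HUD's buff panel.
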(event `self.ReceiveBeginPlay`
  (`parent.ReceiveBeginPlay`)
  (`self.ClearDuplicate`))

(event `self.ReceiveEndPlay`
  (params (EndPlayReason :type "EEndPlayReason Enum" :default "Destroyed")))

(fn `CastAbility`
  (`/Game/SubSystems/Ability/UI/WBP_BuffPanel.AddBuffToUI` (`/Game/Base/WBP_Player_UI.WBP_BuffPanel` (`/Game/Base/BP_Player_HUD.PlayerUI_Ref` (`/Game/Base/BFL_BasicFunctions.Get Player HUD`))) self))

(fn `ClearDuplicate`
  (bind (_abilityinfo_abilityclass _abilityinfo_abilityname _abilityinfo_abilitydescription _abilityinfo_abilitytype _abilityinfo_ispassive _abilityinfo_abilityeffect) (break `/Game/SubSystems/Ability/SystemFiles/S_AbilityInfo` (`self.AbilityInfo`)))
  (for _array_element (`self.GetAttachedActors` (`self.GetOwner`) true)
    (if (== (`GameplayStatics.GetObjectClass` _array_element) (`GameplayStatics.GetObjectClass` self))
      (`/Game/SubSystems/PlayerStats/SystemFiles/AC_CharacterStats.BuffCleared` (`/Game/Base/BFL_BasicFunctions.GetPlayerStatsSubsystem`) _abilityinfo_abilityeffect)
      (`self.K2_DestroyActor` _array_element))))

(fn `OnNotification`
  (params (NotificationName :type Name :default "None"))
  (switch `name` NotificationName
    (:`CastAbility`
      (`self.CastAbility`))))

(fn `UserConstructionScript`
  (`parent.UserConstructionScript`))