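; Ranged fireball ability actor that launches as a projectile and explodes on overlap with any actor except its owner.
; Notifications start its particle emitter and cast it, detaching the actor and activating projectile movement.
; On overlap it spawns an explosion, applies full radial damage from AbilityInfo within four times the sphere radius, sparing the owner, and destroys itself.
; It also resets player movement to Walking and leaves debug print and sphere drawing.
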(event `self.Sphere.OnComponentBeginOverlap`
  (params (OverlappedComponent :type "PrimitiveComponent Object Reference") (OtherActor :type "Actor Object Reference") (OtherComp :type "PrimitiveComponent Object Reference") (OtherBodyIndex :type Integer) (bFromSweep :type Boolean) (SweepResult :type "HitResult Structure (by ref)"))
  (if (not (== (`self.GetOwner`) OtherActor))
    (`KismetSystemLibrary.PrintString` (`KismetSystemLibrary.GetDisplayName` OtherActor))
    (`self.ApplyAbilityEffect`)
    (`CharacterMovementComponent.SetMovementMode` (`Character.CharacterMovement` (`/Game/Base/BFL_BasicFunctions.GetPlayerCharacter`)) "MOVE_Walking" 0)))

(fn `ActivateAbility`
  (`self.K2_DetachFromActor` "KeepWorld" "KeepRelative" "KeepWorld")
  (`ActorComponent.Activate` (`self.ProjectileMovement`) false))

(fn `ApplyAbilityEffect`
  (bind _sphere (`self.Sphere`))
  (bind _returnvalue (`SceneComponent.K2_GetComponentLocation` _sphere))
  (bind _returnvalue_2 (* (`SphereComponent.SphereRadius` _sphere) 4.0))
  (`KismetSystemLibrary.DrawDebugSphere` _returnvalue _returnvalue_2 12 (struct :`R` 1.0 :`G` 1.0 :`B` 1.0 :`A` 1.0) 10.0 2.0)
  (`GameplayStatics.SpawnEmitterAtLocation` "/Game/Assets/FXVarietyPack/Particles/P_ky_explosion.P_ky_explosion" _returnvalue)
  (`GameplayStatics.ApplyRadialDamage` (`KismetMathLibrary.Conv_IntToDouble` (`.DamageToInflict_18_A24E7FF144F7319C6F5067A84845BCAD` (break `/Game/SubSystems/Ability/SystemFiles/S_AbilityEffect` (`.AbilityEffect_17_9A09C93F49D390455C9DFA863FD069DA` (break `/Game/SubSystems/Ability/SystemFiles/S_AbilityInfo` (`self.AbilityInfo`)))))) _returnvalue _returnvalue_2 null (`|MakeArray` (`self.GetOwner`)) null null true)
  (`self.K2_DestroyActor`))

(fn `OnNotification`
  (params (NotificationName :type Name))
  (switch `name` NotificationName
    (:`StartEmitter`
      (`ActorComponent.Activate` (`self.ParticleSystem`) false))
    (:`CastAbility`
      (`self.ActivateAbility`))))

(fn `UserConstructionScript`)