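; Ability system component that casts the abilities in the player's left and right mouse slots and feeds them to the HUD icons.
; UseAbility picks a slot by mouse button; attack abilities first move to the cast target via the player controller.
; Casting stops movement, faces the cursor hit and spawns the ability actor behind a DoOnce.
; Cast completion restores walking and resets the gate; repeat input while casting clears the busy flag after a short delay.
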(event `SetAbilities`
  (bind _mainskills (`/Game/SubSystems/PlayerStats/UI/WBP_PlayerMainHud_UI.MainSkills` (`/Game/Base/WBP_Player_UI.WBP_PlayerMainHud_UI` (`/Game/Base/BP_Player_HUD.PlayerUI_Ref` (`/Game/Base/BFL_BasicFunctions.Get Player HUD`)))))
  (set `/Game/SubSystems/Ability/SystemFiles/Base/UI/WBP_AbilityIcon.AbilityRef` (`self.LeftSlotAbility`) (`/Game/SubSystems/Ability/SystemFiles/Base/UI/WBP_AbilityBar.WBP_AbilityIconLeft` _mainskills))
  (set `/Game/SubSystems/Ability/SystemFiles/Base/UI/WBP_AbilityIcon.AbilityRef` (`self.RightSlotAbility`) (`/Game/SubSystems/Ability/SystemFiles/Base/UI/WBP_AbilityBar.WBP_AbilityIconRight` _mainskills)))

(event `self.ReceiveBeginPlay`
  (bind _ascharacter (cast `Character` (`self.GetOwner`)))
  (set `self.Owner` _ascharacter))

(event `UseAbility`
  (params (Key :type "Key Structure" :default "None"))
  (bind _player_controller (`/Game/Base/BFL_BasicFunctions.GetPlayerController`))
  (bind _ability (`self.Ability`))
  (bind _owner (`self.Owner`))
  (bind (_returnvalue_roll _returnvalue_pitch) (`KismetMathLibrary.BreakRotator` (`Actor.K2_GetActorRotation` _owner)))
  (bind (_returnvalue_roll_2 _returnvalue_pitch_2 _returnvalue_yaw) (`KismetMathLibrary.BreakRotator` (`KismetMathLibrary.FindLookAtRotation` (`Actor.K2_GetActorLocation` _owner) (`.Location` (`GameplayStatics.BreakHitResult` (`PlayerController.GetHitResultUnderCursorByChannel` (`/Game/Base/BFL_BasicFunctions.GetPlayerController`) "TraceTypeQuery1" true))))))
  (if (`self.CastingInProgress`)
    (`KismetSystemLibrary.Delay` 0.2)
    (set `self.CastingInProgress` false)
    (else
      (set `self.CastingInProgress` true)
      (if (== Key "LeftMouseButton")
        (set `self.Ability` (`self.LeftSlotAbility`))
        (if (`.bSuccess` (castclass `/Game/SubSystems/Ability/SystemFiles/Base/System/BP_Ability_Attack` _ability :!pure true)) :!label _label
          (add `/Game/Base/BP_PlayerController.TargetReached` _player_controller (delegate `SpawnAbility`))
          (`/Game/Base/BP_PlayerController.MoveToCastTarget` _player_controller)
          (else
            (`/Engine/EditorBlueprintResources/StandardMacros.DoOnce` false :!label _label_2
              (:`Completed`
                (`CharacterMovementComponent.DisableMovement` (`Character.CharacterMovement` (`/Game/Base/BFL_BasicFunctions.GetPlayerCharacter`)))
                (`Actor.K2_SetActorRotation` _owner (`KismetMathLibrary.MakeRotator` _returnvalue_roll _returnvalue_pitch _returnvalue_yaw) false)
                (bind _returnvalue (`|SpawnActorFromClass` _ability (`Actor.GetTransform` (`self.Owner`)) "Undefined" "OverrideRootScale" (`self.Owner`) null))
                (`/Game/SubSystems/Ability/SystemFiles/Base/System/BP_BaseAbility.BeginCasting` _returnvalue)
                (add `/Game/SubSystems/Ability/SystemFiles/Base/System/BP_BaseAbility.CastComplete` _returnvalue (delegate `Reset`))))))
        (elif (== Key "RightMouseButton")
          (set `self.Ability` (`self.RightSlotAbility`))
          (goto _label)
          (else
            (set `self.CastingInProgress` false)))))))

(event `SpawnAbility`
  (goto _label_2))

(event `Reset`
  (`CharacterMovementComponent.SetMovementMode` (`Character.CharacterMovement` (`/Game/Base/BFL_BasicFunctions.GetPlayerCharacter`)) "MOVE_Walking" 0)
  (set `self.CastingInProgress` false)
  (goto _label_2 :!via `Reset`))