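; Base ability component that handles montage-driven casting for a character's abilities.
; On BeginPlay it loads its details from a data table row, then snaps itself to a socket on the owning Character's mesh.
; BeginCasting reattaches and plays the cast montage on the player character if none is playing, firing CastComplete on completion or blend out.
; Montage notifies and interruption of interruptable casts only print debug strings.
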(event `self.ReceiveBeginPlay`
  (bind (_abilitydetailsdth_datatable _abilitydetailsdth_rowname) (break `DataTableRowHandle` (`self.AbilityDetailsDTH`)))
  (bind _returnvalue (`|GetDataTableRow` _abilitydetailsdth_datatable _abilitydetailsdth_rowname)
    (:`then`
      (set `self.AbilityDetails` _returnvalue)
      (`self.AttachToSocket`))))

(event `BeginCasting`
  (bind _mesh (`Character.Mesh` (`/Game/Base/BFL_BasicFunctions.GetPlayerCharacter`)))
  (`self.AttachToSocket`)
  (`KismetSystemLibrary.PrintString` "Casting")
  (if (not (`AnimInstance.IsAnyMontagePlaying` (`SkeletalMeshComponent.GetAnimInstance` _mesh)))
    (bind _notifyname (`|PlayMontage` _mesh (`self.AbilityCastMontage`))
      (:`OnCompleted`
        (`self.CastComplete` :!label _label)
        (`KismetSystemLibrary.PrintString` "Complete"))
      (:`OnBlendOut`
        (goto _label))
      (:`OnNotifyBegin`
        (`self.OnNotifyBegin` _notifyname)))))

(fn `AttachToSocket`
  (bind _ascharacter (cast `Character` (`self.GetOwner`)))
  (`self.K2_AttachToComponent` self (`Character.Mesh` _ascharacter) (`self.SocketToAttach`) "SnapToTarget" "SnapToTarget" "SnapToTarget" true))

(fn `OnCastInterrupted`
  (if (and (== (`Character.GetCurrentMontage` (`/Game/Base/BFL_BasicFunctions.GetPlayerCharacter`)) (`self.AbilityCastMontage`)) (`.IsInterruptable_18_B125FB2E4382C067A19732A4EA903A1C` (break `/Game/SubSystems/Ability/SystemFiles/Base/System/S_AbilityDetails` (`self.AbilityDetails`))))
    (`KismetSystemLibrary.PrintString` "Interrupted")))

(fn `OnNotifyBegin`
  (params (NotifyName :type Name))
  (`KismetSystemLibrary.PrintString` (`KismetStringLibrary.Concat_StrStr` "Notify \"" (`KismetStringLibrary.Conv_NameToString` NotifyName) "\" reached")))

(fn `UserConstructionScript`)