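; Ability component that builds the character's skill book, triggers abilities and toggles the skill book widget on the HUD.
; On BeginPlay it fills AvailableAbilities from DT_Abilities and runs a basic-ability pass over LearnedAbilities that cannot add anything.
; UseAbility spawns the ability's actor, attaches it to the character mesh and activates it.
; Starter-equip and left-button logic is disconnected; the right-button handler disables movement and calls UseAbility without an ability.
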(event `self.ReceiveBeginPlay`
  (`self.BuildSkillBook`)
  (`self.SetBasicAbilities`))

(fn `BuildSkillBook`
  (bind _outrownames (`DataTableFunctionLibrary.GetDataTableRowNames` "/Game/SubSystems/Ability/SystemFiles/DT_Abilities.DT_Abilities"))
  (for _array_element _outrownames
    (bind _returnvalue (`|GetDataTableRow` "/Game/SubSystems/Ability/SystemFiles/DT_Abilities.DT_Abilities" _array_element)
      (:`then`
        (`KismetArrayLibrary.Array_AddUnique` (`self.AvailableAbilities`) _returnvalue)))))

(fn `EquipStarterAbilities`)

(fn `OpenSkillBook`
  (bind _skillbookref (`self.SkillBookRef`)
    (:`then`
      (`Widget.RemoveFromParent` _skillbookref)
      (set `self.SkillBookRef` null))
    (:`else`
      (bind _returnvalue (`|CreateWidget` "/Game/SubSystems/Ability/UI/WBP_Skillbook.WBP_SkillBook_C"))
      (bind _output_get (set `self.SkillBookRef` _returnvalue))
      (bind _returnvalue_2 (`CanvasPanel.AddChildToCanvas` (`/Game/Base/WBP_Player_UI.SkillBookCanvas` (`/Game/Base/BP_Player_HUD.PlayerUI_Ref` (`/Game/Base/BFL_BasicFunctions.Get Player HUD`))) _output_get))
      (`CanvasPanelSlot.SetAutoSize` _returnvalue_2 true))))

(fn `SetBasicAbilities`
  (bind _learnedabilities (`self.LearnedAbilities`))
  (for _array_element (`self.LearnedAbilities`)
    (if (and (not (`KismetArrayLibrary.Array_Contains` _learnedabilities _array_element)) (`|EnumEquality` (`.AbilityType_10_9208DFE344939450854AA8BDEE0F0997` (break `/Game/SubSystems/Ability/SystemFiles/S_AbilityInfo` _array_element)) "NewEnumerator3"))
      (`KismetArrayLibrary.Array_AddUnique` _learnedabilities _array_element))))

(fn `UseAbility`
  (params (AbilityToUse :type "/Game/SubSystems/Ability/SystemFiles/S_AbilityInfo Structure"))
  (bind _returnvalue (`self.GetOwner`))
  (bind _returnvalue_2 (`|SpawnActorFromClass` (`.AbilityClass_4_DDFE158B4E29B80684CCDD8326275496` (break `/Game/SubSystems/Ability/SystemFiles/S_AbilityInfo` AbilityToUse)) (`Actor.GetTransform` _returnvalue) "Undefined" "SelectDefaultAtRuntime" _returnvalue null))
  (`Actor.K2_AttachToComponent` _returnvalue_2 (`Character.Mesh` (cast `Character` _returnvalue :!pure true)) "None" "SnapToTarget" "SnapToTarget" "SnapToTarget" true)
  (`/Game/SubSystems/Ability/SystemFiles/BP_AbilityBase.UseAbility` _returnvalue_2))

(fn `UseSkillLeftButton`)

(fn `UseSkillRightButton`
  (bind _charactermovement (`Character.CharacterMovement` (`/Game/Base/BFL_BasicFunctions.GetPlayerCharacter`)))
  (`MovementComponent.StopMovementImmediately` _charactermovement)
  (`CharacterMovementComponent.DisableMovement` _charactermovement)
  (`self.UseAbility` (struct)))