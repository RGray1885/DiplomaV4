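; Inventory component that stores the player's items as stacked item structs and handles pickup, dropping, use and the inventory screen toggle.
; Adds merge into a stack with room or append; removals match the stored index, falling back to a class search.
; Aid items apply data-table effects through the player stats subsystem, while equipment spawns and equips.
; Quick slots read their items directly from HUD widgets, and dispatchers announce most inventory changes.
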(fn `AddToInventory`
  (params (ItemToAdd :type "/Game/SubSystems/Inventory/SystemFiles/S_ItemInfo Structure"))
  (locals (FoundItemStruct :type "/Game/SubSystems/Inventory/SystemFiles/S_ItemInfo Structure") (bItemFound :type Boolean) (FoundItemIndex :type Integer))
  (bind (_itemclass _itemname _itemdescription _itemtype _itemcurrentamount) (break `/Game/SubSystems/Inventory/SystemFiles/S_ItemInfo` ItemToAdd))
  (bind (_itemclass_2 _itemname_2 _itemdescription_2 _itemtype_2 _itemcurrentamount_2 _itemstacksize _itemprice _equipmentinfo _aiditeminfo _icon _iteminventoryindex) (break `/Game/SubSystems/Inventory/SystemFiles/S_ItemInfo` ItemToAdd))
  (bind (_itemclass_3 _itemname_3 _itemdescription_3 _itemtype_3 _itemcurrentamount_3 _itemstacksize_2 _itemprice_2 _equipmentinfo_2 _aiditeminfo_2 _icon_2) (break `/Game/SubSystems/Inventory/SystemFiles/S_ItemInfo` ItemToAdd))
  (bind _inventory (`self.Inventory`))
  (for (_array_element _array_index) (`self.Inventory`)
    (bind (_itemclass_4 _itemname_4 _itemdescription_4 _itemtype_4 _itemcurrentamount_4 _itemstacksize_3) (break `/Game/SubSystems/Inventory/SystemFiles/S_ItemInfo` _array_element))
    (if (and (== _itemclass_4 _itemclass) (<= (+ _itemcurrentamount_4 _itemcurrentamount) _itemstacksize_3))
      (set `local.bItemFound` true)
      (set `local.FoundItemStruct` _array_element)
      (set `local.FoundItemIndex` _array_index)
      (break)))
  (if (`local.bItemFound`)
    (`KismetArrayLibrary.Array_Set` (`self.Inventory`) (`local.FoundItemIndex`) (make `/Game/SubSystems/Inventory/SystemFiles/S_ItemInfo` _itemclass_2 _itemname_2 _itemdescription_2 _itemtype_2 (+ (`.ItemCurrentAmount_13_DEDDED7742D3C5B674192CB07820D4CE` (break `/Game/SubSystems/Inventory/SystemFiles/S_ItemInfo` (`local.FoundItemStruct`))) _itemcurrentamount_2) _itemstacksize _itemprice _equipmentinfo _aiditeminfo _icon _iteminventoryindex))
    (`KismetSystemLibrary.PrintString` "+1 to existing")
    (else
      (`KismetArrayLibrary.Array_Add` _inventory (make `/Game/SubSystems/Inventory/SystemFiles/S_ItemInfo` _itemclass_3 _itemname_3 _itemdescription_3 _itemtype_3 _itemcurrentamount_3 _itemstacksize_2 _itemprice_2 _equipmentinfo_2 _aiditeminfo_2 _icon_2 (+ (`KismetArrayLibrary.Array_LastIndex` _inventory) 1)))
      (`KismetSystemLibrary.PrintString` "New item added")))
  (`self.InventoryRefreshed`))

(fn `DropItem`
  (params (ItemToDrop :type "/Game/SubSystems/Inventory/SystemFiles/S_ItemInfo Structure"))
  (bind (_itemclass _itemname _itemdescription _itemtype _itemcurrentamount _itemstacksize _itemprice _equipmentinfo _aiditeminfo _icon _iteminventoryindex) (break `/Game/SubSystems/Inventory/SystemFiles/S_ItemInfo` ItemToDrop))
  (`|SpawnActorFromClass` _itemclass (`KismetMathLibrary.MakeTransform` (`Actor.K2_GetActorLocation` (`self.GetOwner`))) "Undefined" "OverrideRootScale" null null)
  (`self.RemoveFromInventory` (make `/Game/SubSystems/Inventory/SystemFiles/S_ItemInfo` _itemclass _itemname _itemdescription _itemtype 1 _itemstacksize _itemprice _equipmentinfo _aiditeminfo _icon _iteminventoryindex)))

(fn `FindAmountOf`
  (params (ItemClass :type "/Game/SubSystems/Inventory/Items/BP_ItemBase Class Reference"))
  (returns (TotalAmountInInventory :type Integer))
  (locals (TotalAmount :type Integer))
  (for _array_element (`self.Inventory`)
    (bind (_itemclass _itemname _itemdescription _itemtype _itemcurrentamount) (break `/Game/SubSystems/Inventory/SystemFiles/S_ItemInfo` _array_element))
    (if (== _itemclass ItemClass)
      (set `local.TotalAmount` (+ (`local.TotalAmount`) _itemcurrentamount))))
  (return (`local.TotalAmount`)))

(fn `OpenInventoryScreen`
  (bind _inventory_ui (`self.Inventory_UI`)
    (:`then`
      (`Widget.RemoveFromParent` _inventory_ui)
      (set `self.Inventory_UI` null))
    (:`else`
      (bind _returnvalue (`|CreateWidget` "/Game/SubSystems/Inventory/UI/WBP_Inventory_UI.WBP_Inventory_UI_C"))
      (bind _output_get (set `self.Inventory_UI` _returnvalue))
      (bind _returnvalue_2 (`CanvasPanel.AddChildToCanvas` (`/Game/Base/WBP_Player_UI.InventoryCanvas` (`/Game/Base/BP_Player_HUD.PlayerUI_Ref` (`/Game/Base/BFL_BasicFunctions.Get Player HUD`))) _output_get))
      (`CanvasPanelSlot.SetAutoSize` _returnvalue_2 true))))

(fn `PickUpItem`
  (params (ItemToPickUp :type "/Game/SubSystems/Inventory/Items/BP_ItemBase Object Reference"))
  (locals (bItemFound :type Boolean) (FoundItemStruct :type "/Game/SubSystems/Inventory/SystemFiles/S_ItemInfo Structure") (FoundItemIndex :type Integer))
  (bind _inventory (`self.Inventory`))
  (bind (_itemclass _itemname _itemdescription _itemtype _itemcurrentamount _itemstacksize _itemprice _equipmentinfo _aiditeminfo _icon _iteminventoryindex) (break `/Game/SubSystems/Inventory/SystemFiles/S_ItemInfo` (`local.FoundItemStruct`)))
  (bind _iteminfo (`/Game/SubSystems/Inventory/SystemFiles/AC_ItemInfoComponent.ItemInfo` (`/Game/SubSystems/Inventory/Items/BP_ItemBase.ItemInfoComponent` ItemToPickUp)))
  (bind (_itemclass_2 _itemname_2 _itemdescription_2 _itemtype_2 _itemcurrentamount_2) (break `/Game/SubSystems/Inventory/SystemFiles/S_ItemInfo` _iteminfo))
  (bind (_itemclass_3 _itemname_3 _itemdescription_3 _itemtype_3 _itemcurrentamount_3 _itemstacksize_2 _itemprice_2 _equipmentinfo_2 _aiditeminfo_2 _icon_2) (break `/Game/SubSystems/Inventory/SystemFiles/S_ItemInfo` _iteminfo))
  (bind (_itemclass_4 _itemname_4 _itemdescription_4 _itemtype_4 _itemcurrentamount_4 _itemstacksize_3 _itemprice_3 _equipmentinfo_3 _aiditeminfo_3 _icon_3) (break `/Game/SubSystems/Inventory/SystemFiles/S_ItemInfo` _iteminfo))
  (bind _s_iteminfo (make `/Game/SubSystems/Inventory/SystemFiles/S_ItemInfo` _itemclass_4 _itemname_4 _itemdescription_4 _itemtype_4 _itemcurrentamount_4 _itemstacksize_3 _itemprice_3 _equipmentinfo_3 _aiditeminfo_3 _icon_3 (+ (`KismetArrayLibrary.Array_LastIndex` _inventory) 1)))
  (for (_array_element _array_index) (`self.Inventory`)
    (bind (_itemclass_5 _itemname_5 _itemdescription_5 _itemtype_5 _itemcurrentamount_5 _itemstacksize_4) (break `/Game/SubSystems/Inventory/SystemFiles/S_ItemInfo` _array_element))
    (if (and (== _itemclass_5 _itemclass_2) (<= (+ _itemcurrentamount_5 _itemcurrentamount_2) _itemstacksize_4))
      (set `local.bItemFound` true)
      (set `local.FoundItemStruct` _array_element)
      (set `local.FoundItemIndex` _array_index)
      (break)))
  (if (`local.bItemFound`)
    (`KismetArrayLibrary.Array_Set` (`self.Inventory`) (`local.FoundItemIndex`) (make `/Game/SubSystems/Inventory/SystemFiles/S_ItemInfo` _itemclass_3 _itemname_3 _itemdescription_3 _itemtype_3 (+ _itemcurrentamount _itemcurrentamount_3) _itemstacksize_2 _itemprice_2 _equipmentinfo_2 _aiditeminfo_2 _icon_2 _iteminventoryindex))
    (`KismetSystemLibrary.PrintString` "+1 to existing")
    (else
      (`KismetArrayLibrary.Array_Add` _inventory _s_iteminfo)
      (`KismetSystemLibrary.PrintString` "New item added")
      (`self.EquipmentPickedUp` _s_iteminfo)))
  (`self.InventoryRefreshed`)
  (`Actor.K2_DestroyActor` ItemToPickUp))

(fn `RemoveFromInventory`
  (params (ItemToRemove :type "/Game/SubSystems/Inventory/SystemFiles/S_ItemInfo Structure"))
  (locals (ItemFound :type Boolean) (FoundItemInfo :type "/Game/SubSystems/Inventory/SystemFiles/S_ItemInfo Structure") (FoundItemIndex :type Integer))
  (bind (_itemclass _itemname _itemdescription _itemtype _itemcurrentamount _itemstacksize _itemprice _equipmentinfo _aiditeminfo _icon _iteminventoryindex) (break `/Game/SubSystems/Inventory/SystemFiles/S_ItemInfo` ItemToRemove))
  (bind _inventory (`self.Inventory`))
  (bind _inventory_2 (`self.Inventory`))
  (bind (_itemclass_2 _itemname_2 _itemdescription_2 _itemtype_2 _itemcurrentamount_2 _itemstacksize_2 _itemprice_2 _equipmentinfo_2 _aiditeminfo_2 _icon_2 _iteminventoryindex_2) (break `/Game/SubSystems/Inventory/SystemFiles/S_ItemInfo` (`local.FoundItemInfo`)))
  (bind (_itemclass_3 _itemname_3 _itemdescription_3 _itemtype_3 _itemcurrentamount_3 _itemstacksize_3 _itemprice_3 _equipmentinfo_3 _aiditeminfo_3 _icon_3 _iteminventoryindex_3) (break `/Game/SubSystems/Inventory/SystemFiles/S_ItemInfo` (`|GetArrayItem` _inventory _iteminventoryindex)))
  (bind _returnvalue (- _itemcurrentamount_2 (`.ItemCurrentAmount_13_DEDDED7742D3C5B674192CB07820D4CE` (break `/Game/SubSystems/Inventory/SystemFiles/S_ItemInfo` ItemToRemove))))
  (bind _returnvalue_2 (- _itemcurrentamount_3 _itemcurrentamount))
  (if (`KismetArrayLibrary.Array_IsValidIndex` _inventory _iteminventoryindex_3)
    (if (== _itemclass_3 _itemclass)
      (if (> _returnvalue_2 0)
        (`KismetArrayLibrary.Array_Set` _inventory _iteminventoryindex_3 (make `/Game/SubSystems/Inventory/SystemFiles/S_ItemInfo` _itemclass_3 _itemname_3 _itemdescription_3 _itemtype_3 _returnvalue_2 _itemstacksize_3 _itemprice_3 _equipmentinfo_3 _aiditeminfo_3 _icon_3 _iteminventoryindex_3))
        (else
          (`KismetArrayLibrary.Array_Remove` _inventory _iteminventoryindex_3)))
      (`self.InventoryRefreshed`)
      (else
        (for (_array_element _array_index) (`self.Inventory`)
          (if (== (`.ItemClass_9_D0CE3054490C15AB80261FA45DC1E5FA` (break `/Game/SubSystems/Inventory/SystemFiles/S_ItemInfo` _array_element)) (`.ItemClass_9_D0CE3054490C15AB80261FA45DC1E5FA` (break `/Game/SubSystems/Inventory/SystemFiles/S_ItemInfo` ItemToRemove)))
            (set `local.FoundItemInfo` _array_element)
            (set `local.FoundItemIndex` _array_index)
            (set `local.ItemFound` true)
            (break)))
        (if (`local.ItemFound`)
          (if (<= _returnvalue 0)
            (`KismetArrayLibrary.Array_Remove` _inventory_2 (`local.FoundItemIndex`))
            (else
              (`KismetArrayLibrary.Array_Set` _inventory_2 (`local.FoundItemIndex`) (make `/Game/SubSystems/Inventory/SystemFiles/S_ItemInfo` _itemclass_2 _itemname_2 _itemdescription_2 _itemtype_2 _returnvalue _itemstacksize_2 _itemprice_2 _equipmentinfo_2 _aiditeminfo_2 _icon_2 _iteminventoryindex_2)))))))))

(fn `SetQuickSlotItems`
  (bind _quickslotitems (`self.QuickSlotItems`))
  (bind _quickslots (`/Game/SubSystems/PlayerStats/UI/WBP_PlayerMainHud_UI.QuickSlots` (`/Game/Base/WBP_Player_UI.WBP_PlayerMainHud_UI` (`/Game/Base/BP_Player_HUD.PlayerUI_Ref` (`/Game/Base/BFL_BasicFunctions.Get Player HUD`)))))
  (`KismetArrayLibrary.Array_Clear` _quickslotitems)
  (`KismetArrayLibrary.Array_Add` _quickslotitems (`/Game/SubSystems/Inventory/UI/WBP_QuickSlotIcon.ItemInfo` (`/Game/SubSystems/PlayerStats/UI/WBP_Player_QuickSlots.QuickSlot1` _quickslots)))
  (`KismetArrayLibrary.Array_Add` _quickslotitems (`/Game/SubSystems/Inventory/UI/WBP_QuickSlotIcon.ItemInfo` (`/Game/SubSystems/PlayerStats/UI/WBP_Player_QuickSlots.QuickSlot2` _quickslots)))
  (`KismetArrayLibrary.Array_Add` _quickslotitems (`/Game/SubSystems/Inventory/UI/WBP_QuickSlotIcon.ItemInfo` (`/Game/SubSystems/PlayerStats/UI/WBP_Player_QuickSlots.Quickslot3` _quickslots)))
  (`KismetArrayLibrary.Array_Add` _quickslotitems (`/Game/SubSystems/Inventory/UI/WBP_QuickSlotIcon.ItemInfo` (`/Game/SubSystems/PlayerStats/UI/WBP_Player_QuickSlots.Quickslot4` _quickslots))))

(fn `UseItemFromInventory`
  (params (ItemToUse :type "/Game/SubSystems/Inventory/SystemFiles/S_ItemInfo Structure"))
  (bind (_itemclass _itemname _itemdescription _itemtype _itemcurrentamount _itemstacksize _itemprice _equipmentinfo _aiditeminfo _icon _iteminventoryindex) (break `/Game/SubSystems/Inventory/SystemFiles/S_ItemInfo` ItemToUse))
  (bind (_datatable _rowname) (break `DataTableRowHandle` _aiditeminfo))
  (bind (_datatable_2 _rowname_2) (break `DataTableRowHandle` _equipmentinfo))
  (bind _s_iteminfo (make `/Game/SubSystems/Inventory/SystemFiles/S_ItemInfo` _itemclass _itemname _itemdescription _itemtype 1 _itemstacksize _itemprice _equipmentinfo _aiditeminfo _icon _iteminventoryindex))
  (switch `/Game/SubSystems/Inventory/SystemFiles/E_ItemType` _itemtype
    (:`NewEnumerator0`
      (bind _returnvalue (`|GetDataTableRow` _datatable _rowname)
        (:`then`
          (bind (_aiditemclass _itemeffect _effectpotency _effectduration) (break `/Game/SubSystems/Inventory/SystemFiles/S_AidItemInfo` _returnvalue))
          (`/Game/SubSystems/PlayerStats/SystemFiles/AC_CharacterStats.ApplyItemEffect` (`/Game/Base/BFL_BasicFunctions.GetPlayerStatsSubsystem`) _itemeffect _effectpotency _effectduration)
          (`self.RemoveFromInventory` _s_iteminfo))))
    (:`NewEnumerator2`
      (bind _returnvalue_2 (`|GetDataTableRow` _datatable_2 _rowname_2)
        (:`then`
          (bind _returnvalue_3 (`|SpawnActorFromClass` (`.EquipmentClass_2_4DD88FF2403FBF68A1ACF88CD044EF53` (break `/Game/SubSystems/Inventory/SystemFiles/S_EquipmentInfo` _returnvalue_2)) (`KismetMathLibrary.MakeTransform` (`Actor.K2_GetActorLocation` (`self.GetOwner`))) "Undefined" "OverrideRootScale" null _s_iteminfo null))
          (`/Game/SubSystems/Inventory/SystemFiles/AC_EquipmentComponent.EquipTo` (`/Game/Base/BP_Player.PlayerEquipment` (`/Game/Base/BFL_BasicFunctions.GetPlayerCharacter`)) _returnvalue_3))))))

(fn `UseQuickSlotItem`
  (params (ItemToUse :type "/Game/SubSystems/Inventory/SystemFiles/S_ItemInfo Structure") (QuickSlot :type "Key Structure" :default "None"))
  (locals (ItemSelector :type Integer) (ItemClassToUse :type "/Game/SubSystems/Inventory/Items/BP_ItemBase Class Reference"))
  (bind _returnvalue (`KismetTextLibrary.Conv_TextToString` (`KismetInputLibrary.Key_GetDisplayName` QuickSlot)))
  (bind _quickslots (`/Game/SubSystems/PlayerStats/UI/WBP_PlayerMainHud_UI.QuickSlots` (`/Game/Base/WBP_Player_UI.WBP_PlayerMainHud_UI` (`/Game/Base/BP_Player_HUD.PlayerUI_Ref` (`/Game/Base/BFL_BasicFunctions.Get Player HUD`)))))
  (bind _quickslot1 (`/Game/SubSystems/PlayerStats/UI/WBP_Player_QuickSlots.QuickSlot1` _quickslots))
  (bind _quickslot2 (`/Game/SubSystems/PlayerStats/UI/WBP_Player_QuickSlots.QuickSlot2` _quickslots))
  (bind _quickslot3 (`/Game/SubSystems/PlayerStats/UI/WBP_Player_QuickSlots.Quickslot3` _quickslots))
  (bind _quickslot4 (`/Game/SubSystems/PlayerStats/UI/WBP_Player_QuickSlots.Quickslot4` _quickslots))
  (bind _returnvalue_2 (select `int` (`local.ItemSelector`) :`0` (`/Game/SubSystems/Inventory/UI/WBP_QuickSlotIcon.ItemInfo` _quickslot1) :`1` (`/Game/SubSystems/Inventory/UI/WBP_QuickSlotIcon.ItemInfo` _quickslot2) :`2` (`/Game/SubSystems/Inventory/UI/WBP_QuickSlotIcon.ItemInfo` _quickslot3) :`3` (`/Game/SubSystems/Inventory/UI/WBP_QuickSlotIcon.ItemInfo` _quickslot4)))
  (`KismetSystemLibrary.PrintString` _returnvalue)
  (switch `string` _returnvalue
    (:`1`
      (set `local.ItemSelector` 0))
    (:`2`
      (set `local.ItemSelector` 1))
    (:`3`
      (set `local.ItemSelector` 2))
    (:`4`
      (set `local.ItemSelector` 3)))
  (set `local.ItemClassToUse` (`.ItemClass_9_D0CE3054490C15AB80261FA45DC1E5FA` (break `/Game/SubSystems/Inventory/SystemFiles/S_ItemInfo` _returnvalue_2)))
  (if (`KismetSystemLibrary.IsValidClass` (`local.ItemClassToUse`))
    (`self.UseItemFromInventory` _returnvalue_2)
    (for _index (range 4)
      (`/Game/SubSystems/Inventory/UI/WBP_QuickSlotIcon.SetButton` (select `int` _index :`0` _quickslot1 :`1` _quickslot2 :`2` _quickslot3 :`3` _quickslot4)))))