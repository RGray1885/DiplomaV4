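; Trader component that holds an NPC shop's stock and handles buying and selling with the player.
; On BeginPlay it seeds stock from DT_Items using StarterInventory counts, then binds to the player inventory's buy and sell events.
; Trades move items between inventories, stacking by class and addressing stock by stored index, which is not refreshed after removals.
; OpenTradeScreen toggles WBP_TradeScreen on the player HUD's trader canvas.
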(event `self.ReceiveBeginPlay`
  (bind _playerinventory (`/Game/Base/BP_Player.PlayerInventory` (`/Game/Base/BFL_BasicFunctions.GetPlayerCharacter`)))
  (`self.FillStarterInventory`)
  (add `/Game/SubSystems/Inventory/SystemFiles/AC_Inventory.SellItem` _playerinventory (`|CreateDelegate` :!event `SellItem`))
  (add `/Game/SubSystems/Inventory/SystemFiles/AC_Inventory.BuyItem` _playerinventory (`|CreateDelegate` :!event `BuyItem`)))

(fn `AddToStock`
  (params (ItemToAdd :type "/Game/SubSystems/Inventory/SystemFiles/S_ItemInfo Structure"))
  (locals (FoundItemIndex :type Integer) (FoundItemInfo :type "/Game/SubSystems/Inventory/SystemFiles/S_ItemInfo Structure") (FoundItem :type Boolean))
  (bind (_itemclass _itemname _itemdescription _itemtype _itemcurrentamount) (break `/Game/SubSystems/Inventory/SystemFiles/S_ItemInfo` ItemToAdd))
  (bind _traderinventory (`self.TraderInventory`))
  (bind (_itemclass_2 _itemname_2 _itemdescription_2 _itemtype_2 _itemcurrentamount_2 _itemstacksize _itemprice _equipmentinfo _aiditeminfo _icon _iteminventoryindex) (break `/Game/SubSystems/Inventory/SystemFiles/S_ItemInfo` (`|GetArrayItem` _traderinventory (`local.FoundItemIndex`))))
  (for (_array_element _array_index) (`self.TraderInventory`)
    (bind (_itemclass_3 _itemname_3 _itemdescription_3 _itemtype_3 _itemcurrentamount_3 _itemstacksize_2) (break `/Game/SubSystems/Inventory/SystemFiles/S_ItemInfo` _array_element))
    (if (and (<= (+ _itemcurrentamount_3 _itemcurrentamount) _itemstacksize_2) (== _itemclass_3 _itemclass))
      (set `local.FoundItemIndex` _array_index)
      (set `local.FoundItemInfo` _array_element)
      (set `local.FoundItem` true)
      (break)))
  (if (not (`local.FoundItem`))
    (bind _returnvalue (`KismetArrayLibrary.Array_Add` _traderinventory ItemToAdd))
    (bind (_itemclass_4 _itemname_4 _itemdescription_4 _itemtype_4 _itemcurrentamount_4 _itemstacksize_3 _itemprice_2 _equipmentinfo_2 _aiditeminfo_2 _icon_2) (break `/Game/SubSystems/Inventory/SystemFiles/S_ItemInfo` (`|GetArrayItem` _traderinventory _returnvalue)))
    (`KismetArrayLibrary.Array_Set` _traderinventory _returnvalue (make `/Game/SubSystems/Inventory/SystemFiles/S_ItemInfo` _itemclass_4 _itemname_4 _itemdescription_4 _itemtype_4 _itemcurrentamount_4 _itemstacksize_3 _itemprice_2 _equipmentinfo_2 _aiditeminfo_2 _icon_2 _returnvalue))
    (else
      (`KismetArrayLibrary.Array_Set` _traderinventory (`local.FoundItemIndex`) (make `/Game/SubSystems/Inventory/SystemFiles/S_ItemInfo` _itemclass_2 _itemname_2 _itemdescription_2 _itemtype_2 (+ _itemcurrentamount_2 (`.ItemCurrentAmount_13_DEDDED7742D3C5B674192CB07820D4CE` (break `/Game/SubSystems/Inventory/SystemFiles/S_ItemInfo` ItemToAdd))) _itemstacksize _itemprice _equipmentinfo _aiditeminfo _icon _iteminventoryindex)))))

(fn `BuyItem`
  (params (ItemToBuy :type "/Game/SubSystems/Inventory/SystemFiles/S_ItemInfo Structure"))
  (`/Game/SubSystems/Inventory/SystemFiles/AC_Inventory.AddToInventory` (`/Game/Base/BP_Player.PlayerInventory` (`/Game/Base/BFL_BasicFunctions.GetPlayerCharacter`)) ItemToBuy)
  (`self.RemoveFromStock` ItemToBuy)
  (`self.TradeComplete`))

(fn `FillStarterInventory`
  (bind _outrownames (`DataTableFunctionLibrary.GetDataTableRowNames` "/Game/SubSystems/Inventory/SystemFiles/DT_Items.DT_Items"))
  (for _array_element _outrownames
    (bind _returnvalue (`|GetDataTableRow` "/Game/SubSystems/Inventory/SystemFiles/DT_Items.DT_Items" _array_element)
      (:`then`
        (bind (_value _returnvalue_2) (`BlueprintMapLibrary.Map_Find` (`self.StarterInventory`) (`.ItemClass_9_D0CE3054490C15AB80261FA45DC1E5FA` (break `/Game/SubSystems/Inventory/SystemFiles/S_ItemInfo` _returnvalue))))
        (if _returnvalue_2
          (for _ (range 1 (+ _value 1))
            (`self.AddToStock` _returnvalue))
          (`self.SetStockIndexes`))))))

(fn `OpenTradeScreen`
  (bind _tradescreenui (`self.TradeScreenUI`)
    (:`then`
      (`Widget.RemoveFromParent` _tradescreenui)
      (set `self.TradeScreenUI` null))
    (:`else`
      (bind _returnvalue (`|CreateWidget` "/Game/SubSystems/Inventory/UI/WBP_TradeScreen.WBP_TradeScreen_C" null self))
      (bind _output_get (set `self.TradeScreenUI` _returnvalue))
      (bind _returnvalue_2 (`CanvasPanel.AddChildToCanvas` (`/Game/Base/WBP_Player_UI.TraderScreenCanvas` (`/Game/Base/BP_Player_HUD.PlayerUI_Ref` (`/Game/Base/BFL_BasicFunctions.Get Player HUD`))) _output_get))
      (`CanvasPanelSlot.SetAutoSize` _returnvalue_2 true))))

(fn `RemoveFromStock`
  (params (ItemToRemove :type "/Game/SubSystems/Inventory/SystemFiles/S_ItemInfo Structure"))
  (locals (FoundItem :type "/Game/SubSystems/Inventory/SystemFiles/S_ItemInfo Structure") (FoundItemIndex :type Integer) (bFoundItem :type Boolean))
  (bind _traderinventory (`self.TraderInventory`))
  (bind (_itemclass _itemname _itemdescription _itemtype _itemcurrentamount _itemstacksize _itemprice _equipmentinfo _aiditeminfo _icon _iteminventoryindex) (break `/Game/SubSystems/Inventory/SystemFiles/S_ItemInfo` (`|GetArrayItem` _traderinventory ItemToRemove_ItemInventoryIndex_42_0EA690824C6D74690E65D3B7679CED7C)))
  (bind _returnvalue (- _itemcurrentamount ItemToRemove_ItemCurrentAmount_13_DEDDED7742D3C5B674192CB07820D4CE))
  (`KismetArrayLibrary.Array_Set` _traderinventory _iteminventoryindex (make `/Game/SubSystems/Inventory/SystemFiles/S_ItemInfo` _itemclass _itemname _itemdescription _itemtype _returnvalue _itemstacksize _itemprice _equipmentinfo _aiditeminfo _icon _iteminventoryindex))
  (if (<= _returnvalue 0)
    (`KismetArrayLibrary.Array_Remove` _traderinventory _iteminventoryindex)))

(fn `SellItem`
  (params (ItemToSell :type "/Game/SubSystems/Inventory/SystemFiles/S_ItemInfo Structure"))
  (`/Game/SubSystems/Inventory/SystemFiles/AC_Inventory.RemoveFromInventory` (`/Game/Base/BP_Player.PlayerInventory` (`/Game/Base/BFL_BasicFunctions.GetPlayerCharacter`)) ItemToSell)
  (`self.AddToStock` ItemToSell)
  (`self.TradeComplete`))

(fn `SetStockIndexes`
  (bind _traderinventory (`self.TraderInventory`))
  (for (_array_element _array_index) _traderinventory
    (bind (_itemclass _itemname _itemdescription _itemtype _itemcurrentamount _itemstacksize _itemprice _equipmentinfo _aiditeminfo _icon) (break `/Game/SubSystems/Inventory/SystemFiles/S_ItemInfo` _array_element))
    (`KismetArrayLibrary.Array_Set` _traderinventory _array_index (make `/Game/SubSystems/Inventory/SystemFiles/S_ItemInfo` _itemclass _itemname _itemdescription _itemtype _itemcurrentamount _itemstacksize _itemprice _equipmentinfo _aiditeminfo _icon _array_index))))