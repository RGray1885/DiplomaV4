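; Base item actor that the player can pick up into their inventory.
; PickUpItem checks the player character's distance to the item; within range, it clears the retry timer and passes itself to the character's PlayerInventory.
; Out of range, it calls CheckDistance on the player controller and re-triggers itself through a very short one-shot timer, polling until the player is close enough.
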(event `/Game/SubSystems/Inventory/Interfaces/BPI_InventoryInteraction.PickUpItem`
  (bind _playercharacter (`/Game/Base/BFL_BasicFunctions.GetPlayerCharacter`))
  ;[1 1 1] Pick up item, add to player's inventory
  (if (<= (`KismetMathLibrary.Vector_Distance` (`self.K2_GetActorLocation` _playercharacter) (`self.K2_GetActorLocation`)) 200.0)
    (`KismetSystemLibrary.K2_ClearAndInvalidateTimerHandle` (`self.DistanceCheckerTimer`))
    (`/Game/SubSystems/Inventory/SystemFiles/AC_Inventory.PickUpItem` (`/Game/Base/BP_Player.PlayerInventory` _playercharacter) self)
    (else
      (`/Game/Base/BP_PlayerController.CheckDistance` (`/Game/Base/BFL_BasicFunctions.GetPlayerController`))
      (bind _returnvalue (`KismetSystemLibrary.K2_SetTimerDelegate` (delegate `/Game/SubSystems/Inventory/Interfaces/BPI_InventoryInteraction.PickUpItem`) 0.001))
      (set `self.DistanceCheckerTimer` _returnvalue))))

(fn `UserConstructionScript`)