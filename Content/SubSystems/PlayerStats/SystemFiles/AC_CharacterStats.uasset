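; Player character stats component that derives combat stats and resource pools, and toggles the stats window on the HUD.
; On BeginPlay it computes damage, defense, attack rate and HP, mana and stamina maximums from attributes, skill bonuses and averaged equipment bonuses.
; Stamina drain and regen use self-rescheduling timers tied to running, calling EffectApplied on changes.
; Item effects only implement health restore; other restore and fortify functions are empty stubs.
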(event `self.ReceiveBeginPlay`
  (bind _asbp_player (cast `/Game/Base/BP_Player` (`self.GetOwner`)))
  (set `self.Player Equipment Ref` (`/Game/Base/BP_Player.PlayerEquipment` _asbp_player))
  (`self.CalculateBaseStats`)
  (set `self.HPCurrent` (/ (`self.HPMax`) 2.0))
  (set `self.ManaCurrent` (/ (`self.ManaMax`) 2.0))
  (set `self.StaminaCurrent` (`self.StaminaMax`)))

(fn `ApplyItemEffect`
  (params (ItemEffect :type "/Game/SubSystems/Inventory/SystemFiles/E_AidItemEffect Enum" :default "NewEnumerator0") (EffectPotency :type Integer) (EffectDuration :type "Float (double-precision)"))
  (locals (EffectTimer :type "TimerHandle Structure"))
  (switch `/Game/SubSystems/Inventory/SystemFiles/E_AidItemEffect` ItemEffect
    (:`NewEnumerator0`
      (`self.RestoreHealth` EffectPotency)
      (`self.EffectApplied`))))

(fn `CalculateBaseStats`
  (locals (FinalDamageBonus :type "Float (double-precision)" :default 0.0) (FinalDefenseBonus :type "Float (double-precision)" :default 0.0))
  (bind _vitality (`self.Vitality`))
  (bind (_equipdamagebonusmin _equipdamagebonusmax _equipdefensebonusmin _equipdefensebonusmax) (`/Game/SubSystems/Inventory/SystemFiles/AC_EquipmentComponent.GetSummarizedStats` (`self.Player Equipment Ref`)))
  (bind _output_get (set `local.FinalDamageBonus` (/ (+ (`KismetMathLibrary.Conv_IntToDouble` _equipdamagebonusmin) (`KismetMathLibrary.Conv_IntToDouble` _equipdamagebonusmax)) 2.0)))
  (bind _output_get_2 (set `local.FinalDefenseBonus` (/ (+ (`KismetMathLibrary.Conv_IntToDouble` _equipdefensebonusmin) (`KismetMathLibrary.Conv_IntToDouble` _equipdefensebonusmax)) 2.0)))
  (`|ExecutionSequence`
    (:`then_0`
      (bind _returnvalue (/ (* _output_get (+ (`KismetMathLibrary.Conv_IntToDouble` (`self.Dexterity`)) 0.75)) 100.0))
      (bind _returnvalue_2 (+ (/ (* _output_get (+ (`KismetMathLibrary.Conv_IntToDouble` (`self.Strength`)) 1.0)) 100.0) _returnvalue (/ (`self.SkillDamageBonus`) 100.0)))
      ;[1 1 1] Damage Calculation
      (set `self.DamageMin` (* _returnvalue_2 0.5))
      (set `self.DamageMax` _returnvalue_2))
    (:`then_1`
      ;[1 1 1] Defense calculation
      (set `self.Defense` (+ (/ (`self.SkillDefenseBonus`) 100.0) (+ (/ _output_get_2 100.0) _returnvalue))))
    (:`then_2`
      ;[1 1 1] HP, stamina, mana calculation
      (set `self.StaminaMax` (`KismetMathLibrary.Conv_IntToDouble` (* _vitality 4))))
    (:`then_3`
      (set `self.HPMax` (`KismetMathLibrary.Conv_IntToDouble` (* _vitality 2))))
    (:`then_4`
      (set `self.ManaMax` (`KismetMathLibrary.Conv_IntToDouble` (`self.Energy`))))
    (:`then_5`
      ;[1 1 1] AttackRate calculation
      (set `self.AttackRate` (`KismetMathLibrary.Conv_IntToDouble` (* (`self.Dexterity`) 4))))))

(fn `DrainStamina`
  (locals (DrainTimer :type "TimerHandle Structure"))
  (bind _playercharacter (`/Game/Base/BFL_BasicFunctions.GetPlayerCharacter`))
  (bind _staminacurrent (`self.StaminaCurrent`))
  (bind _isrunning (`/Game/Base/BP_Player.IsRunning` _playercharacter))
  (if _isrunning
    (if (<= _staminacurrent 0.0)
      (`KismetSystemLibrary.K2_ClearAndInvalidateTimerHandle` (`local.DrainTimer`) :!label _label)
      (`/Game/Base/BP_Player.Run` _playercharacter _isrunning)
      (else
        (`KismetSystemLibrary.PrintString` "DrainingStamina")
        (bind _output_get (set `self.StaminaCurrent` (`KismetMathLibrary.FClamp` (- _staminacurrent (`self.StaminaDrain`)) 0.0 (`self.StaminaMax`))))
        (`self.EffectApplied`)
        (if (<= _output_get 0.0)
          (goto _label)
          (else
            (bind _returnvalue (`KismetSystemLibrary.K2_SetTimer` null "DrainStamina" (`self.StaminaRegenRate`)))
            (set `local.DrainTimer` _returnvalue)))))))

(fn `FortifyHealth`
  (params (EffectPotency :type Integer)))

(fn `FortifyMana`
  (params (EffectPotency :type Integer)))

(fn `FortifyStamina`
  (params (EffectPotency :type Integer)))

(fn `OpenStatsScreen`
  (bind _statswindowref (`self.StatsWindowRef`)
    (:`then`
      (`Widget.RemoveFromParent` _statswindowref)
      (set `self.StatsWindowRef` null))
    (:`else`
      (bind _returnvalue (`|CreateWidget` "/Game/SubSystems/PlayerStats/UI/WBP_PlayerStats.WBP_PlayerStats_C" null self))
      (bind _output_get (set `self.StatsWindowRef` _returnvalue))
      (bind _returnvalue_2 (`CanvasPanel.AddChildToCanvas` (`/Game/Base/WBP_Player_UI.StatsCanvas` (`/Game/Base/BP_Player_HUD.PlayerUI_Ref` (`/Game/Base/BFL_BasicFunctions.Get Player HUD`))) _output_get))
      (`CanvasPanelSlot.SetAutoSize` _returnvalue_2 true))))

(fn `RegenStamina`
  (locals (StaminaRegenTimer :type "TimerHandle Structure"))
  (if (not (`/Game/Base/BP_Player.IsRunning` (`/Game/Base/BFL_BasicFunctions.GetPlayerCharacter`)))
    (`KismetSystemLibrary.PrintString` "RegenStarted")
    (set `self.StaminaCurrent` (`KismetMathLibrary.FClamp` (+ (`self.StaminaCurrent`) (`self.StaminaRegenAmount`)) 0.0 (`self.StaminaMax`)))
    (if (>= (`self.StaminaCurrent`) (`self.StaminaMax`))
      (`KismetSystemLibrary.K2_ClearAndInvalidateTimerHandle` (`local.StaminaRegenTimer`))
      (else
        (bind _returnvalue (`KismetSystemLibrary.K2_SetTimer` null "RegenStamina" (`self.StaminaRegenRate`)))
        (set `local.StaminaRegenTimer` _returnvalue)))
    (`self.EffectApplied`)))

(fn `RestoreHealth`
  (params (EffectPotency :type Integer))
  (bind _hpcurrent (`self.HPCurrent`))
  (set `self.HPCurrent` (`KismetMathLibrary.FClamp` (+ (`KismetMathLibrary.Conv_IntToDouble` EffectPotency) _hpcurrent) _hpcurrent (`self.HPMax`))))

(fn `RestoreMana`
  (params (EffectPotency :type Integer)))

(fn `RestoreStamina`
  (params (EffectPotency :type Integer)))