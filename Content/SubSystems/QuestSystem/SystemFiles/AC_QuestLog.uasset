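; AC_QuestLog is a quest log component that tracks a list of quest IDs and their spawned BP_Quest_Base actors.
; AddQuest records the ID, spawns and stores a quest actor, then calls the still-empty GetCollectionObjectives.
; CompleteQuest flags and destroys matching actors without removing them from either list.
; TrackQuest can only clear the active quest so far, and objective, turn-in and reward functions are empty stubs.
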(fn `AddQuest`
  (params (QuestID :type Name))
  (`KismetArrayLibrary.Array_AddUnique` (`self.AvailableQuests`) QuestID)
  (bind _returnvalue (`|SpawnActorFromClass` "/Game/SubSystems/QuestSystem/SystemFiles/BP_Quest_Base.BP_Quest_Base_C" (`KismetMathLibrary.MakeTransform` (0.0 0.0 0.0)) "Undefined" "OverrideRootScale" null QuestID null))
  (`KismetArrayLibrary.Array_Add` (`self.CurrentQuests`) _returnvalue)
  (bind _questdetails_questname (break `/Game/SubSystems/QuestSystem/SystemFiles/S_QuestDetails` (`/Game/SubSystems/QuestSystem/SystemFiles/BP_Quest_Base.QuestDetails` _returnvalue)))
  (`KismetSystemLibrary.PrintString` (`KismetStringLibrary.Concat_StrStr` "Quest " (`KismetTextLibrary.Conv_TextToString` _questdetails_questname) " spawned and added"))
  (`self.GetCollectionObjectives`))

(fn `CheckMoveToObjective`)

(fn `CompleteObjective`)

(fn `CompleteQuest`
  (params (QuestID :type Name))
  (if (`self.QueryActiveQuest` QuestID)
    (for _array_element (`self.CurrentQuests`)
      (if (== (`/Game/SubSystems/QuestSystem/SystemFiles/BP_Quest_Base.QuestID` _array_element) QuestID)
        (set `/Game/SubSystems/QuestSystem/SystemFiles/BP_Quest_Base.IsComplete` true _array_element)
        (`Actor.K2_DestroyActor` _array_element)))))

(fn `FindLocationObjective`)

(fn `FindRequiredQuest`)

(fn `GetAmountForCollectionObjective`)

(fn `GetCollectionObjectives`)

(fn `GetCurrentActiveQuest`)

(fn `QueryActiveQuest`
  (params (QuestID :type Name))
  (returns (ReturnValue :type Boolean))
  (return (`KismetArrayLibrary.Array_Contains` (`self.AvailableQuests`) QuestID)))

(fn `ReceiveStageRewards`)

(fn `TrackQuest`
  (params (QuestID :type Name))
  (if (== QuestID (`self.ActiveQuest`))
    (set `self.ActiveQuest` "None")
    (elif (`self.QueryActiveQuest` QuestID)
      _)))

(fn `TurnInStageQuest`)