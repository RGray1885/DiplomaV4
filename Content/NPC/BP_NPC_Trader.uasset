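; BP_NPC_Trader is a trader NPC that opens its trade screen once the player character is close enough.
; Tradewith measures the distance to the player and, when in range, clears the polling timer and calls OpenTradeScreen on TraderComponent.
; When out of range, it calls CheckDistance on the player controller and sets a very short one-shot timer on a trade event, apparently itself, to poll until the player arrives.
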(event `/Game/SubSystems/Inventory/Interfaces/BPI_Trader.TradeWith`
  (if (<= (`KismetMathLibrary.Vector_Distance` (`self.K2_GetActorLocation` (`/Game/Base/BFL_BasicFunctions.GetPlayerCharacter`)) (`self.K2_GetActorLocation`)) 200.0)
    (`KismetSystemLibrary.K2_ClearAndInvalidateTimerHandle` (`self.DistanceCheckerTimer`))
    (`/Game/SubSystems/Inventory/SystemFiles/AC_Trader.OpenTradeScreen` (`self.TraderComponent`))
    (else
      (`/Game/Base/BP_PlayerController.CheckDistance` (`/Game/Base/BFL_BasicFunctions.GetPlayerController`))
      (bind _returnvalue (`KismetSystemLibrary.K2_SetTimerDelegate` (delegate `/Game/SubSystems/Inventory/Interfaces/BPI_Trader.TradeWith`) 0.001))
      (set `self.DistanceCheckerTimer` _returnvalue))))

(fn `UserConstructionScript`
  (`parent.UserConstructionScript`))