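; BP_Player is the player character Blueprint, with a sprint ability gated by stamina.
; BeginPlay caches the default walk speed, and Run doubles it and starts PlayerStats stamina drain when sprinting is requested with stamina remaining.
; Otherwise Run restores the default speed, calling stamina regeneration only when sprint is not requested.
; Stamina is checked only when Run is called.
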(event `self.ReceiveBeginPlay`
  (set `self.DefaultMaxSpeed` (`CharacterMovementComponent.MaxWalkSpeed` (`self.CharacterMovement`))))

(fn `Run`
  (params (`ShouldRun?` :type Boolean))
  (locals (DrainTimer :type "TimerHandle Structure") (TimerLoop :type Boolean) (RegenTimer :type "TimerHandle Structure"))
  (bind _playerstats (`self.PlayerStats`))
  (bind _charactermovement (`self.CharacterMovement`))
  (bind _output_get (set `self.IsRunning` `ShouldRun?`))
  (if _output_get
    (if (<= (`/Game/SubSystems/PlayerStats/SystemFiles/AC_CharacterStats.StaminaCurrent` _playerstats) 0.0)
      (set `CharacterMovementComponent.MaxWalkSpeed` (`self.DefaultMaxSpeed`) _charactermovement :!label _label)
      (if (not (`self.IsRunning`))
        (`/Game/SubSystems/PlayerStats/SystemFiles/AC_CharacterStats.RegenStamina` _playerstats))
      (else
        (set `CharacterMovementComponent.MaxWalkSpeed` (* (`self.DefaultMaxSpeed`) 2.0) _charactermovement)
        (`/Game/SubSystems/PlayerStats/SystemFiles/AC_CharacterStats.DrainStamina` _playerstats)))
    (else
      (goto _label))))

(fn `UserConstructionScript`)