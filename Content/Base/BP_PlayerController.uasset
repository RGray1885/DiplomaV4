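; Player controller for click-to-move control of the character, plus hotkeys for running, mouse-wheel zoom, inventory, stats, a quick slot and skills.
; Holding left mouse, or calling MoveToCastTarget, traces under the cursor and applies movement input toward the hit location.
; A re-armed short timer keeps the character moving until within MinClickDistance.
; On arrival it sends pickup and trade messages to the clicked actor, or faces an Enemy-tagged one and fires TargetReached.
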(event `self.ReceiveTick`
  (params (DeltaSeconds :type "Float (single-precision)"))
  (bind _playercharacter (`/Game/Base/BFL_BasicFunctions.GetPlayerCharacter`))
  (bind _playercharacter_2 (`/Game/Base/BFL_BasicFunctions.GetPlayerCharacter`))
  (bind _clicklocation (`self.ClickLocation`))
  (bind (_bblockinghit _binitialoverlap _time _distance _location _impactpoint _normal _impactnormal _physmat _hitactor) (`GameplayStatics.BreakHitResult` (`self.GetHitResultUnderCursorByChannel` "TraceTypeQuery1")))
  (bind _returnvalue (`self.K2_GetActorLocation` _playercharacter))
  (bind (_returnvalue_roll _returnvalue_pitch) (`KismetMathLibrary.BreakRotator` (`self.K2_GetActorRotation` _playercharacter_2)))
  (bind _returnvalue_2 (`KismetMathLibrary.FindLookAtRotation` _returnvalue _clicklocation))
  (bind _returnvalue_3 (`KismetMathLibrary.VSize` (- _returnvalue _clicklocation)))
  (`/Engine/EditorBlueprintResources/StandardMacros.Gate` true :!label _label
    (:`Exit`
      (set `self.ClickLocation` _location :!label _label_2)
      (bind _output_get (set `self.ClickActor` _hitactor))
      (if (>= _returnvalue_3 (`self.MinClickDistance`))
        (`Pawn.AddMovementInput` _playercharacter (`KismetMathLibrary.GetDirectionUnitVector` _returnvalue _clicklocation) _returnvalue_3 false)
        (if (== _returnvalue _clicklocation :`ErrorTolerance` (`self.MinClickDistance`)) :!label _label_3
          (`KismetSystemLibrary.K2_ClearAndInvalidateTimerHandle` (`self.MoveToTimer`))
          (`|ExecutionSequence`
            (:`then_0`
              (message `/Game/SubSystems/Inventory/Interfaces/BPI_InventoryInteraction.PickUpItem` _output_get))
            (:`then_1`
              (`/Engine/EditorBlueprintResources/StandardMacros.IsValid` _output_get
                (:`Is Valid`
                  (message `/Game/SubSystems/Inventory/Interfaces/BPI_Trader.TradeWith` _output_get))))
            (:`then_2`
              (`/Engine/EditorBlueprintResources/StandardMacros.IsValid` _output_get
                (:`Is Valid`
                  (if (`self.ActorHasTag` _output_get "Enemy")
                    (`self.K2_SetActorRotation` _playercharacter_2 (`KismetMathLibrary.MakeRotator` _returnvalue_roll _returnvalue_pitch (.yaw _returnvalue_2)) false)
                    (`self.TargetReached`))))))
          (else
            (`Pawn.AddMovementInput` _playercharacter (`KismetMathLibrary.GetForwardVector` _returnvalue_2) _returnvalue_3 false)
            (bind _returnvalue_4 (`KismetSystemLibrary.K2_SetTimerDelegate` (delegate `CheckDistance`) 0.001))
            (set `self.MoveToTimer` _returnvalue_4)))))))

(event `MoveToCastTarget`
  (goto _label_2))

(event `Key|LeftMouseButton`
  (params (Key :type "Key Structure"))
  (:`Pressed`
    (goto _label :!via `Open`))
  (:`Released`
    (goto _label :!via `Close`)))

(event `CheckDistance`
  (goto _label_3))

(event `Key|I`
  (params (Key :type "Key Structure"))
  (:`Pressed`
    (`/Game/SubSystems/Inventory/SystemFiles/AC_Inventory.OpenInventoryScreen` (`/Game/Base/BP_Player.PlayerInventory` (`/Game/Base/BFL_BasicFunctions.GetPlayerCharacter`)))))

(event `InputAxisKey|MouseWheelAxis`
  (params (AxisValue :type "Float (single-precision)"))
  (bind _springarm (`/Game/Base/BP_Player.SpringArm` (`/Game/Base/BFL_BasicFunctions.GetPlayerCharacter`)))
  (set `SpringArmComponent.TargetArmLength` (+ (* AxisValue -50.0) (`SpringArmComponent.TargetArmLength` _springarm)) _springarm))

(event `Key|C`
  (params (Key :type "Key Structure"))
  (:`Pressed`
    (`/Game/SubSystems/PlayerStats/SystemFiles/AC_CharacterStats.OpenStatsScreen` (`/Game/Base/BP_Player.PlayerStats` (`/Game/Base/BFL_BasicFunctions.GetPlayerCharacter`)))))

(event `Key|One`
  (params (Key :type "Key Structure"))
  (:`Pressed`
    (`/Game/SubSystems/Inventory/SystemFiles/AC_Inventory.UseQuickSlotItem` :`self` (`/Game/Base/BFL_BasicFunctions.GetPlayerInventorySubsystem`) :`QuickSlot` Key)))

(event `Key|LeftControl`
  (params (Key :type "Key Structure"))
  (bind _playercharacter (`/Game/Base/BFL_BasicFunctions.GetPlayerCharacter`))
  (:`Pressed`
    (`/Game/Base/BP_Player.Run` _playercharacter true))
  (:`Released`
    (`/Game/Base/BP_Player.Run` _playercharacter false)))

(event `InputAction|UseSkill`
  (params (Key :type "Key Structure"))
  (:`Pressed`
    (`/Game/SubSystems/Ability/SystemFiles/Base/System/AC_AbilitySystemComponent.UseAbility` (`/Game/Base/BFL_BasicFunctions.GetPlayerAbilitySubsystem`) Key)))

(fn `UserConstructionScript`)